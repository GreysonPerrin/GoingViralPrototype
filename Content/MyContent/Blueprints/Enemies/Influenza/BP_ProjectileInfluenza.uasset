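; BP_ProjectileInfluenza is a homing enemy projectile that chases the player and can be shot down.
; On BeginPlay it caches the game instance and sets the player character, cast to BP_PlayerController, as its ProjectileMovement homing target.
; Collision overlaps with player bullets destroy the bullet and reduce Health, and at zero it reports a defeat to the game instance and destroys itself.
; Touching the player deals damage without destroying the projectile.
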(event OnComponentBeginOverlap(Collision)
  (params (OverlappedComponent :type Primitive%20Component%20Object%20Reference) (OtherActor :type Actor%20Object%20Reference) (OtherComp :type Primitive%20Component%20Object%20Reference) (OtherBodyIndex :type Integer) (bFromSweep :type Boolean) (SweepResult :type Hit%20Result%20Structure%20%28by%20ref%29))
  ;[0.15 0.15 0.15 0.5] Damaged when hit by bullet
  (Utilities|Casting|CastToBP_PlayerBullet OtherActor
    (:then
      (Actor|DestroyActor OtherActor)
      (Variables|Default|SetHealth (- (Variables|Default|GetHealth) 1.0))
      (if (not (> (Variables|Default|GetHealth) 0.0))
        (Default|DefeatEnemy (Variables|Default|GetBP%20Game%20Instance) 1 1)
        (Actor|DestroyActor)))
    (:CastFailed
      ;[0.15 0.15 0.15 0.5] Damage player on contact
      (bind _asbp_player_controller (Utilities|Casting|CastToBP_PlayerController OtherActor))
      (Default|TakeDamage _asbp_player_controller 2))))

(event EventBeginPlay
  (bind _asbp_game_instance (Utilities|Casting|CastToBP_GameInstance (Game|GetGameInstance)))
  (Variables|Default|SetBP%20Game%20Instance _asbp_game_instance)
  (bind _asbp_player_controller (Utilities|Casting|CastToBP_PlayerController (Game|GetPlayerCharacter 0)))
  ;[0.15 0.15 0.15 0.5] Set player as homing target
  (bind _output_get (Variables|Default|SetBP%20Player%20Controller _asbp_player_controller))
  (Variables|/Script/Engine.ProjectileMovementComponent|SetHomingTargetComponent (Variables|Default|GetProjectileMovement) (Variables|/Script/Engine.Actor|GetRootComponent _output_get)))

(event Collision|EventActorBeginOverlap
  (params (OtherActor :type Actor%20Object%20Reference)))

(event EventTick
  (params (DeltaSeconds :type Float%20%28single-precision%29)))

(fn ConstructionScript)