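; Adenovirus enemy pawn that chases the player and fires bombs at close range.
; Tick runs the chase only while the pawn is within the player's camera range, moving it straight toward the player.
; Inside the distance threshold it spawns four cardinal projectiles on a cooldown, primed to fire immediately on entry.
; Bullet overlaps reduce health and report defeat to the game instance at zero; player contact deals damage.
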(event OnComponentBeginOverlap(Collision)
  (params (OverlappedComponent :type Primitive%20Component%20Object%20Reference) (OtherActor :type Actor%20Object%20Reference) (OtherComp :type Primitive%20Component%20Object%20Reference) (OtherBodyIndex :type Integer) (bFromSweep :type Boolean) (SweepResult :type Hit%20Result%20Structure%20%28by%20ref%29))
  ;[0.15 0.15 0.15 0.5] Damaged when hit by bullet
  (Utilities|Casting|CastToBP_PlayerBullet OtherActor
    (:then
      (Actor|DestroyActor OtherActor)
      (Variables|Default|SetHealth (- (Variables|Default|GetHealth) 1.0))
      (if (not (> (Variables|Default|GetHealth) 0.0))
        (Default|DefeatEnemy (Variables|Default|GetBP%20Game%20Instance) 10 1)
        (Actor|DestroyActor)))
    (:CastFailed
      ;[0.15 0.15 0.15 0.5] Damage the player on contact
      (bind _asbp_player_controller (Utilities|Casting|CastToBP_PlayerController OtherActor))
      (Default|TakeDamage _asbp_player_controller 6))))

(event Custom|Move%20Towards%20Player
  (bind _returnvalue (Transformation|GetActorLocation))
  (bind _cooldown (Variables|Default|GetCooldown))
  (bind _bp_player_controller (Variables|Default|GetBP%20Player%20Controller))
  (bind _returnvalue_2 (Transformation|GetActorLocation _bp_player_controller))
  ;[0.15 0.15 0.15 0.5] Move towards player function
  (Pawn|Input|AddMovementInput (Math|Vector|Normalize (- _returnvalue_2 _returnvalue)) 1.0 false)
  (if (<= (Math|Vector|Distance(Vector) _returnvalue _returnvalue_2) (Variables|Default|GetDistance%20Threshold))
    (CallFunction|PlayerinRange)
    (elif (< (Variables|Default|GetTimer) _cooldown)
      (Variables|Default|SetTimer _cooldown))))

(event Custom|Player%20in%20%20Range
  ;[0.15 0.15 0.15 0.5] Attack the player on a cooldown when they are close enough
  (if (>= (Variables|Default|GetTimer) (Variables|Default|GetCooldown))
    (CallFunction|FireBombs)
    (Variables|Default|SetTimer 0.0)
    (else
      (Variables|Default|SetTimer (+ (Variables|Default|GetTimer) (stale EventTick DeltaSeconds))))))

(event Custom|Fire%20Bombs
  (bind _returnvalue (Transformation|GetActorLocation))
  ;[0.15 0.15 0.15 0.5] Launch bombs in all directions
  (Game|SpawnActorfromClass "/Game/MyContent/Blueprints/Enemies/Adenovirus/BP_ProjectileAdenovirus.BP_ProjectileAdenovirus_C" (Math|Transform|MakeTransform _returnvalue (Math|Conversions|RotationFromXVector (Class|KismetMathLibrary|VectorForward)) "1.000000,1.000000,1.000000") "Undefined" "MultiplyWithRoot" 0 0)
  (Game|SpawnActorfromClass "/Game/MyContent/Blueprints/Enemies/Adenovirus/BP_ProjectileAdenovirus.BP_ProjectileAdenovirus_C" (Math|Transform|MakeTransform _returnvalue (Math|Conversions|RotationFromXVector (Class|KismetMathLibrary|VectorBackward)) "1.000000,1.000000,1.000000") "Undefined" "MultiplyWithRoot" 0 0)
  (Game|SpawnActorfromClass "/Game/MyContent/Blueprints/Enemies/Adenovirus/BP_ProjectileAdenovirus.BP_ProjectileAdenovirus_C" (Math|Transform|MakeTransform _returnvalue (Math|Conversions|RotationFromXVector (Class|KismetMathLibrary|VectorLeft)) "1.000000,1.000000,1.000000") "Undefined" "MultiplyWithRoot" 0 0)
  (Game|SpawnActorfromClass "/Game/MyContent/Blueprints/Enemies/Adenovirus/BP_ProjectileAdenovirus.BP_ProjectileAdenovirus_C" (Math|Transform|MakeTransform _returnvalue (Math|Conversions|RotationFromXVector (Class|KismetMathLibrary|VectorRight)) "1.000000,1.000000,1.000000") "Undefined" "MultiplyWithRoot" 0 0))

(event EventBeginPlay
  (bind _asbp_game_instance (Utilities|Casting|CastToBP_GameInstance (Game|GetGameInstance)))
  (Variables|Default|SetBP%20Game%20Instance _asbp_game_instance)
  (bind _asbp_player_controller (Utilities|Casting|CastToBP_PlayerController (Game|GetPlayerCharacter 0)))
  (Variables|Default|SetBP%20Player%20Controller _asbp_player_controller)
  (Variables|/Script/Engine.FloatingPawnMovement|SetMaxSpeed (Variables|Default|GetFloatingPawnMovement) (Variables|Default|GetMove%20Speed)))

(event Collision|EventActorBeginOverlap
  (params (OtherActor :type Actor%20Object%20Reference)))

(event EventTick
  (params (DeltaSeconds :type Float%20%28single-precision%29))
  (bind _returnvalue (Transformation|GetActorLocation))
  (bind _bp_player_controller (Variables|Default|GetBP%20Player%20Controller))
  (bind _bp_player_controller_2 (Variables|Default|GetBP%20Player%20Controller))
  (bind _returnvalue_2 (Transformation|GetActorLocation _bp_player_controller_2))
  ;[0.15 0.15 0.15 0.5] If enemy is within the camera's range
  (if (and (<= (Math|Float|Absolute(Float) (- (.x _returnvalue) (.x _returnvalue_2))) (Variables|/Game/MyContent/Player/BP_PlayerController.BP_PlayerController_C|GetH%20Camera%20Range _bp_player_controller)) (<= (Math|Float|Absolute(Float) (- (.y _returnvalue) (.y _returnvalue_2))) (Variables|/Game/MyContent/Player/BP_PlayerController.BP_PlayerController_C|GetV%20Camera%20Range _bp_player_controller)))
    (if (Variables|Default|GetOn%20Camera)
      (CallFunction|MoveTowardsPlayer)
      (else
        (Variables|Default|SetOn%20Camera true)))
    (elif (Variables|Default|GetOn%20Camera)
      (Variables|Default|SetOn%20Camera false))))

(fn ConstructionScript)