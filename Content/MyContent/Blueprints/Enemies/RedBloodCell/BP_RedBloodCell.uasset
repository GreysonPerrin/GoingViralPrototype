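; Red blood cell actor in the Enemies set that drifts along the X axis and removes itself on certain overlaps.
; On BeginPlay it sets its ProjectileMovement velocity from MoveSpeed.
; Its Collision overlap destroys it immediately at a BP_BloodCellDespawner.
; Touching a bacteriophage or influenza pawn destroys it one frame later, only if that pawn's OnCamera flag is set.
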(event OnComponentBeginOverlap(Collision)
  (params (OverlappedComponent :type Primitive%20Component%20Object%20Reference) (OtherActor :type Actor%20Object%20Reference) (OtherComp :type Primitive%20Component%20Object%20Reference) (OtherBodyIndex :type Integer) (bFromSweep :type Boolean) (SweepResult :type Hit%20Result%20Structure%20%28by%20ref%29))
  (Utilities|Casting|CastToBP_BloodCellDespawner OtherActor
    (:then
      (Actor|DestroyActor))
    (:CastFailed
      (bind _asbp_pawn_bacteriophage (Utilities|Casting|CastToBP_PawnBacteriophage OtherActor)
        (:then
          (if (Variables|/Game/MyContent/Blueprints/Enemies/Bacteriophage/BP_PawnBacteriophage.BP_PawnBacteriophage_C|GetOn%20Camera _asbp_pawn_bacteriophage)
            (Utilities|FlowControl|DelayUntilNextFrame)
            (Actor|DestroyActor)))
        (:CastFailed
          (bind _asbp_pawn_influenza (Utilities|Casting|CastToBP_PawnInfluenza OtherActor))
          (if (Variables|/Game/MyContent/Blueprints/Enemies/Influenza/BP_PawnInfluenza.BP_PawnInfluenza_C|GetOn%20Camera _asbp_pawn_influenza)
            (Utilities|FlowControl|DelayUntilNextFrame)
            (Actor|DestroyActor)))))))

(event EventBeginPlay
  (bind _result (Math|Float|NegateFloat (Variables|Default|GetMove%20Speed))
    (:%20%20
      (Variables|/Script/Engine.MovementComponent|SetVelocity (Variables|Default|GetProjectileMovement) (Math|Vector|MakeVector _result 0.0 0.0)))))

(event Collision|EventActorBeginOverlap
  (params (OtherActor :type Actor%20Object%20Reference)))

(event EventTick
  (params (DeltaSeconds :type Float%20%28single-precision%29)))

(fn ConstructionScript)