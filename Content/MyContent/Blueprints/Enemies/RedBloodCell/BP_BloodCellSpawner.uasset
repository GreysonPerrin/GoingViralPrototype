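; Spawner actor that fills an area with BP_RedBloodCell actors and keeps adding more during play.
; On BeginPlay it spawns an initial batch at random X and Y offsets around its own location, across a wide field.
; A Tick-driven timer then spawns one cell each interval at the field's positive X edge, with a random Y offset.
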(event Custom|Spawn%20Cell%20Start
  (Game|SpawnActorfromClass "/Game/MyContent/Blueprints/Enemies/RedBloodCell/BP_RedBloodCell.BP_RedBloodCell_C" (Math|Transform|MakeTransform (+ (Transformation|GetActorLocation) (Math|Vector|MakeVector (Math|Random|RandomFloatinRange -1.25e+04 1.25e+04) (Math|Random|RandomFloatinRange -2e+03 3e+03) 0.0)) "0, 0, 0" "1.000000,1.000000,1.000000") "Undefined" "MultiplyWithRoot" 0 0))

(event Custom|Spawn%20Cell%20During
  (Game|SpawnActorfromClass "/Game/MyContent/Blueprints/Enemies/RedBloodCell/BP_RedBloodCell.BP_RedBloodCell_C" (Math|Transform|MakeTransform (+ (Transformation|GetActorLocation) (Math|Vector|MakeVector 1.25e+04 (Math|Random|RandomFloatinRange -2e+03 3e+03) 0.0)) "0, 0, 0" "1.000000,1.000000,1.000000") "Undefined" "MultiplyWithRoot" 0 0))

(event EventBeginPlay
  (for _index (range 0 50)
    (CallFunction|SpawnCellStart)))

(event Collision|EventActorBeginOverlap
  (params (OtherActor :type Actor%20Object%20Reference)))

(event EventTick
  (params (DeltaSeconds :type Float%20%28single-precision%29))
  (bind _output_get (Variables|Default|SetTimer (+ (Variables|Default|GetTimer) DeltaSeconds)))
  (if (>= _output_get (Variables|Default|GetInterval))
    (CallFunction|SpawnCellDuring)
    (Variables|Default|SetTimer 0.0)))

(fn ConstructionScript)