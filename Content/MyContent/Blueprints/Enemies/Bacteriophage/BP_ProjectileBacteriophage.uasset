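; BP_ProjectileBacteriophage is a projectile actor for the Bacteriophage enemy that handles its own despawning.
; On BeginPlay it caches the player character as BP_PlayerController.
; Each tick it destroys itself once its X or Y distance from the player exceeds that character's horizontal or vertical camera range.
; Overlapping the player with its Collision component also destroys it, with no damage applied in this graph.
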(event OnComponentBeginOverlap(Collision)
  (params (OverlappedComponent :type Primitive%20Component%20Object%20Reference) (OtherActor :type Actor%20Object%20Reference) (OtherComp :type Primitive%20Component%20Object%20Reference) (OtherBodyIndex :type Integer) (bFromSweep :type Boolean) (SweepResult :type Hit%20Result%20Structure%20%28by%20ref%29))
  ;[0.15 0.15 0.15 0.5] Despawn after hitting the player
  (Utilities|Casting|CastToBP_PlayerController OtherActor)
  (Actor|DestroyActor))

(event EventBeginPlay
  (bind _asbp_player_controller (Utilities|Casting|CastToBP_PlayerController (Game|GetPlayerCharacter 0)))
  (Variables|Default|SetBP%20Player%20Controller _asbp_player_controller))

(event Collision|EventActorBeginOverlap
  (params (OtherActor :type Actor%20Object%20Reference)))

(event EventTick
  (params (DeltaSeconds :type Float%20%28single-precision%29))
  (bind _returnvalue (Transformation|GetActorLocation))
  (bind _bp_player_controller (Variables|Default|GetBP%20Player%20Controller))
  (bind _bp_player_controller_2 (Variables|Default|GetBP%20Player%20Controller))
  (bind _returnvalue_2 (Transformation|GetActorLocation _bp_player_controller_2))
  ;[0.15 0.15 0.15 0.5] Despawn after going offscreen
  (if (not (and (<= (Math|Float|Absolute(Float) (- (.x _returnvalue) (.x _returnvalue_2))) (Variables|/Game/MyContent/Player/BP_PlayerController.BP_PlayerController_C|GetH%20Camera%20Range _bp_player_controller)) (<= (Math|Float|Absolute(Float) (- (.y _returnvalue) (.y _returnvalue_2))) (Variables|/Game/MyContent/Player/BP_PlayerController.BP_PlayerController_C|GetV%20Camera%20Range _bp_player_controller))))
    (Actor|DestroyActor)))

(fn ConstructionScript)