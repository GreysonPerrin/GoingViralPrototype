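; BP_PawnBacteriophage is an enemy pawn that hunts the nearest red blood cell while within the player's camera range.
; Each tick it checks its distance to the player against the camera extents, then moves and rotates toward that cell via FloatingPawnMovement.
; Player bullets reduce its health and award currency on death.
; Touching a cell while on camera replaces the pawn with an infected bacteriophage enemy.
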(event OnComponentBeginOverlap(Collision)
  (params (OverlappedComponent :type Primitive%20Component%20Object%20Reference) (OtherActor :type Actor%20Object%20Reference) (OtherComp :type Primitive%20Component%20Object%20Reference) (OtherBodyIndex :type Integer) (bFromSweep :type Boolean) (SweepResult :type Hit%20Result%20Structure%20%28by%20ref%29))
  ;[0.15 0.15 0.15 0.5] Damaged when hit by bullet
  (Utilities|Casting|CastToBP_PlayerBullet OtherActor
    (:then
      (Actor|DestroyActor OtherActor)
      (Variables|Default|SetHealth (- (Variables|Default|GetHealth) 1.0))
      (if (not (> (Variables|Default|GetHealth) 0.0))
        (Default|GainCurrency (Variables|Default|GetBP%20Player%20Controller) 5)
        (Actor|DestroyActor)))
    (:CastFailed
      ;[0.15 0.15 0.15 0.5] Infect a red blood cell after touching it
      (Utilities|Casting|CastToBP_RedBloodCell OtherActor)
      (if (Variables|Default|GetOn%20Camera)
        (Game|SpawnActorfromClass "/Game/MyContent/Blueprints/Enemies/Bacteriophage/BP_EnemyBacteriophageInfected.BP_EnemyBacteriophageInfected_C" (Transformation|GetWorldTransform (Variables|Default|GetDefaultSceneRoot)) "Undefined" "MultiplyWithRoot" 0 0)
        (Utilities|FlowControl|DelayUntilNextFrame)
        (Actor|DestroyActor)))))

(event Custom|Move%20Towards%20Cell
  (bind _returnvalue (Transformation|GetActorLocation))
  ;[0.15 0.15 0.15 0.5] Find and move towards the nearest red blood cell
  (bind _outactors (Actor|GetAllActorsOfClass "/Game/MyContent/Blueprints/Enemies/RedBloodCell/BP_RedBloodCell.BP_RedBloodCell_C"))
  (Pawn|Input|AddMovementInput (Math|Vector|MakeVector (.x (Math|Vector|Normalize (- (Transformation|GetActorLocation (.ReturnValue (Actor|FindNearestActor (Transformation|GetActorLocation) _outactors))) _returnvalue))) (.y (Math|Vector|Normalize (- (Transformation|GetActorLocation (.ReturnValue (Actor|FindNearestActor (Transformation|GetActorLocation) _outactors))) _returnvalue))) 0.0) 1.0 true)
  (Transformation|SetActorRotation (Math|Rotator|FindLookatRotation _returnvalue (Transformation|GetActorLocation (.ReturnValue (Actor|FindNearestActor (Transformation|GetActorLocation) _outactors))))))

(event EventBeginPlay
  (bind _asbp_player_controller (Utilities|Casting|CastToBP_PlayerController (Game|GetPlayerCharacter 0)))
  (Variables|Default|SetBP%20Player%20Controller _asbp_player_controller)
  (Variables|/Script/Engine.FloatingPawnMovement|SetMaxSpeed (Variables|Default|GetFloatingPawnMovement) (Variables|Default|GetMove%20Speed)))

(event Collision|EventActorBeginOverlap
  (params (OtherActor :type Actor%20Object%20Reference)))

(event EventTick
  (params (DeltaSeconds :type Float%20%28single-precision%29))
  (bind _returnvalue (Transformation|GetActorLocation))
  (bind _bp_player_controller (Variables|Default|GetBP%20Player%20Controller))
  (bind _bp_player_controller_2 (Variables|Default|GetBP%20Player%20Controller))
  (bind _returnvalue_2 (Transformation|GetActorLocation _bp_player_controller_2))
  ;[0.15 0.15 0.15 0.5] If enemy is within the camera's range
  (if (and (<= (Math|Float|Absolute(Float) (- (.x _returnvalue) (.x _returnvalue_2))) (Variables|/Game/MyContent/Player/BP_PlayerController.BP_PlayerController_C|GetH%20Camera%20Range _bp_player_controller)) (<= (Math|Float|Absolute(Float) (- (.y _returnvalue) (.y _returnvalue_2))) (Variables|/Game/MyContent/Player/BP_PlayerController.BP_PlayerController_C|GetV%20Camera%20Range _bp_player_controller)))
    (if (Variables|Default|GetOn%20Camera)
      (CallFunction|MoveTowardsCell)
      (else
        (Variables|Default|SetOn%20Camera true)))
    (elif (Variables|Default|GetOn%20Camera)
      (Variables|Default|SetOn%20Camera false))))

(fn ConstructionScript)