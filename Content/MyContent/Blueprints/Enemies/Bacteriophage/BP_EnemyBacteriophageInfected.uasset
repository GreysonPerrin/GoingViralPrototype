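; Infected bacteriophage enemy that turns to face the player and fires projectiles while within the player camera's range.
; Tick compares its X/Y offset from the player to the camera ranges, then smoothly rotates and spawns projectiles from ShootPoint on a timer.
; Player bullets deal double damage on the virus body versus the cell; death reports Vitalis and a kill to the game instance.
; Touching the cell also damages the player.
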(event OnComponentBeginOverlap(CellCollision)
  (params (OverlappedComponent :type Primitive%20Component%20Object%20Reference) (OtherActor :type Actor%20Object%20Reference) (OtherComp :type Primitive%20Component%20Object%20Reference) (OtherBodyIndex :type Integer) (bFromSweep :type Boolean) (SweepResult :type Hit%20Result%20Structure%20%28by%20ref%29))
  ;[0.15 0.15 0.15 0.5] Damaged when hit by bullet
  (Utilities|Casting|CastToBP_PlayerBullet OtherActor
    (:then
      (Actor|DestroyActor OtherActor)
      (Variables|Default|SetHealth (- (Variables|Default|GetHealth) 1.0))
      (if (not (> (Variables|Default|GetHealth) 0.0))
        (Default|DefeatEnemy (Variables|Default|GetBP%20Game%20Instance) 5 1)
        (Actor|DestroyActor)))
    (:CastFailed
      ;[0.15 0.15 0.15 0.5] Damage the player on contact
      (bind _asbp_player_controller (Utilities|Casting|CastToBP_PlayerController OtherActor))
      (Default|TakeDamage _asbp_player_controller 1))))

(event OnComponentBeginOverlap(VirusCollision)
  (params (OverlappedComponent :type Primitive%20Component%20Object%20Reference) (OtherActor :type Actor%20Object%20Reference) (OtherComp :type Primitive%20Component%20Object%20Reference) (OtherBodyIndex :type Integer) (bFromSweep :type Boolean) (SweepResult :type Hit%20Result%20Structure%20%28by%20ref%29))
  ;[0.15 0.15 0.15 0.5] Takes double damage if the bacteriophage's body is hit
  (Utilities|Casting|CastToBP_PlayerBullet OtherActor)
  (Actor|DestroyActor OtherActor)
  (Variables|Default|SetHealth (- (Variables|Default|GetHealth) 2.0))
  ;[0.15 0.15 0.15 0.5] Damaged when hit by bullet
  (if (not (> (Variables|Default|GetHealth) 0.0))
    (Default|DefeatEnemy (Variables|Default|GetBP%20Game%20Instance) 5 1)
    (Actor|DestroyActor)))

(event Custom|Face%20Player
  ;[0.15 0.15 0.15 0.5] Turn to face player
  (Transformation|SetActorRotation (Math|Interpolation|RInterpTo (Transformation|GetActorRotation) (Math|Rotator|FindLookatRotation (Transformation|GetActorLocation) (Transformation|GetActorLocation (Variables|Default|GetBP%20Player%20Controller))) (stale EventTick DeltaSeconds) (Variables|Default|GetRotate%20Speed))))

(event Custom|Shooting
  ;[0.15 0.15 0.15 0.5] Shoot at the player at a set interval
  (bind _output_get (Variables|Default|SetTimer (+ (Variables|Default|GetTimer) (stale EventTick DeltaSeconds))))
  (if (>= _output_get (Variables|Default|GetShoot%20Rate))
    (Game|SpawnActorfromClass "/Game/MyContent/Blueprints/Enemies/Bacteriophage/BP_ProjectileBacteriophage.BP_ProjectileBacteriophage_C" (Transformation|GetWorldTransform (Variables|Default|GetShoot%20Point)) "Undefined" "MultiplyWithRoot" 0 0)
    (Variables|Default|SetTimer 0.0)))

(event EventBeginPlay
  (bind _asbp_game_instance (Utilities|Casting|CastToBP_GameInstance (Game|GetGameInstance)))
  (Variables|Default|SetBP%20Game%20Instance _asbp_game_instance)
  (bind _asbp_player_controller (Utilities|Casting|CastToBP_PlayerController (Game|GetPlayerCharacter 0)))
  (Variables|Default|SetBP%20Player%20Controller _asbp_player_controller))

(event Collision|EventActorBeginOverlap
  (params (OtherActor :type Actor%20Object%20Reference)))

(event EventTick
  (params (DeltaSeconds :type Float%20%28single-precision%29))
  (bind _returnvalue (Transformation|GetActorLocation))
  (bind _bp_player_controller (Variables|Default|GetBP%20Player%20Controller))
  (bind _bp_player_controller_2 (Variables|Default|GetBP%20Player%20Controller))
  (bind _returnvalue_2 (Transformation|GetActorLocation _bp_player_controller_2))
  ;[0.15 0.15 0.15 0.5] If enemy is within the camera's range
  (if (and (<= (Math|Float|Absolute(Float) (- (.x _returnvalue) (.x _returnvalue_2))) (Variables|/Game/MyContent/Player/BP_PlayerController.BP_PlayerController_C|GetH%20Camera%20Range _bp_player_controller)) (<= (Math|Float|Absolute(Float) (- (.y _returnvalue) (.y _returnvalue_2))) (Variables|/Game/MyContent/Player/BP_PlayerController.BP_PlayerController_C|GetV%20Camera%20Range _bp_player_controller)))
    (if (Variables|Default|GetOn%20Camera)
      (CallFunction|FacePlayer)
      (CallFunction|Shooting)
      (else
        (Variables|Default|SetOn%20Camera true)))
    (elif (Variables|Default|GetOn%20Camera)
      (Variables|Default|SetOn%20Camera false))))

(fn ConstructionScript)