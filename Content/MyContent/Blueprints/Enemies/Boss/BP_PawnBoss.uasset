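; Boss enemy pawn that chases and faces the player every tick, firing BP_ProjectileBoss from its shoot point on a cooldown while in range.
; Leaving range primes the timer, so it fires immediately when the player is back in range.
; LosePiece tracks health as remaining pieces, triggering phase 2 when few remain and granting currency on death.
; In phase 2, each shot also spawns a minion, cycling through Bacteriophage, Adenovirus and Influenza.
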(event Custom|LosePiece
  ;[0.15 0.15 0.15 0.5] Keeps track of remaining pieces
  (Variables|Default|SetPieces (- (Variables|Default|GetPieces) 1))
  (if (> (Variables|Default|GetPieces) 0)
    (if (and (<= (Variables|Default|GetPieces) 5) (not (Variables|Default|GetPhase%202)))
      (Variables|Default|SetPhase%202 true))
    (else
      (Default|GainCurrency (Variables|Default|GetBP%20Player%20Controller) 30)
      (Actor|DestroyActor))))

(event Custom|Move%20Toward%20Player
  (bind _returnvalue (Transformation|GetActorLocation))
  (bind _bp_player_controller (Variables|Default|GetBP%20Player%20Controller))
  (bind _cooldown (Variables|Default|GetCooldown))
  (bind _returnvalue_2 (Transformation|GetActorLocation _bp_player_controller))
  ;[0.15 0.15 0.15 0.5] Move towards player function
  (Pawn|Input|AddMovementInput (Math|Vector|Normalize (- _returnvalue_2 _returnvalue)) 1.0 false)
  (if (<= (Math|Vector|Distance(Vector) _returnvalue _returnvalue_2) (Variables|Default|GetDistance%20Threshold))
    (CallFunction|PlayerinRange)
    (elif (< (Variables|Default|GetTimer) _cooldown)
      (Variables|Default|SetTimer _cooldown))))

(event Custom|Player%20In%20Range
  ;[0.15 0.15 0.15 0.5] Attack the player on a cooldown if they are close enough
  (if (>= (Variables|Default|GetTimer) (Variables|Default|GetCooldown))
    (CallFunction|FireMetaball)
    (Variables|Default|SetTimer 0.0)
    (else
      (Variables|Default|SetTimer (+ (Variables|Default|GetTimer) (stale EventTick DeltaSeconds))))))

(event Custom|Fire%20Metaball
  (bind _shoot_point (Variables|Default|GetShoot%20Point))
  (bind _returnvalue (Transformation|GetWorldTransform _shoot_point))
  ;[0.15 0.15 0.15 0.5] Attack the player on a cooldown if they are close enough
  (Game|SpawnActorfromClass "/Game/MyContent/Blueprints/Enemies/Boss/BP_ProjectileBoss.BP_ProjectileBoss_C" (Transformation|GetWorldTransform (Variables|Default|GetShoot%20Point)) "Undefined" "MultiplyWithRoot" 0 0)
  (if (Variables|Default|GetPhase%202)
    (switch int (Variables|Default|GetEnemy%20to%20Spawn)
      (:Default
        (Game|SpawnActorfromClass "/Game/MyContent/Blueprints/Enemies/Bacteriophage/BP_PawnBacteriophage.BP_PawnBacteriophage_C" _returnvalue "Undefined" "MultiplyWithRoot" 0 0 :!label _label))
      (:0
        (goto _label))
      (:1
        (Game|SpawnActorfromClass "/Game/MyContent/Blueprints/Enemies/Adenovirus/BP_PawnAdenovirus.BP_PawnAdenovirus_C" _returnvalue "Undefined" "MultiplyWithRoot" 0 0))
      (:2
        (Game|SpawnActorfromClass "/Game/MyContent/Blueprints/Enemies/Influenza/BP_PawnInfluenza.BP_PawnInfluenza_C" _returnvalue "Undefined" "MultiplyWithRoot" 0 0)))
    (bind _result (Math|Integer|IncrementInt (Variables|Default|GetEnemy%20to%20Spawn))
      (:%20%20
        (if (> _result 2)
          (Variables|Default|SetEnemy%20to%20Spawn 0))))))

(event Custom|Turn%20Towards%20Player
  ;[0.15 0.15 0.15 0.5] Turn shoot point towards player
  (Transformation|SetRelativeRotation (Variables|Default|GetCollision) (Math|Rotator|FindLookatRotation (Transformation|GetActorLocation) (Transformation|GetActorLocation (Variables|Default|GetBP%20Player%20Controller))) false false))

(event EventBeginPlay
  (bind _asbp_player_controller (Utilities|Casting|CastToBP_PlayerController (Game|GetPlayerCharacter 0)))
  (Variables|Default|SetBP%20Player%20Controller _asbp_player_controller)
  (Variables|/Script/Engine.FloatingPawnMovement|SetMaxSpeed (Variables|Default|GetFloatingPawnMovement) (Variables|Default|GetMove%20Speed)))

(event Collision|EventActorBeginOverlap
  (params (OtherActor :type Actor%20Object%20Reference)))

(event EventTick
  (params (DeltaSeconds :type Float%20%28single-precision%29))
  (CallFunction|MoveTowardPlayer)
  (CallFunction|TurnTowardsPlayer))

(fn ConstructionScript)