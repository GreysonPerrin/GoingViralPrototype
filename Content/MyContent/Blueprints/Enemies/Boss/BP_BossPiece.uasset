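; BP_BossPiece is a destructible piece of the boss enemy, expecting BP_PawnBoss as its parent actor.
; Collision overlaps with player bullets destroy the bullet and reduce the piece's Health; at zero it calls LosePiece on the boss and destroys itself.
; Other overlaps damage the player on contact through TakeDamage on BP_PlayerController, which BeginPlay treats as the player character despite its name.
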(event OnComponentBeginOverlap(Collision)
  (params (OverlappedComponent :type Primitive%20Component%20Object%20Reference) (OtherActor :type Actor%20Object%20Reference) (OtherComp :type Primitive%20Component%20Object%20Reference) (OtherBodyIndex :type Integer) (bFromSweep :type Boolean) (SweepResult :type Hit%20Result%20Structure%20%28by%20ref%29))
  ;[0.15 0.15 0.15 0.5] Damaged when shot by player
  (Utilities|Casting|CastToBP_PlayerBullet OtherActor
    (:then
      (Actor|DestroyActor OtherActor)
      (Variables|Default|SetHealth (- (Variables|Default|GetHealth) 1.0))
      (if (not (> (Variables|Default|GetHealth) 0.0))
        (Default|LosePiece (Variables|Default|GetBoss%20BP))
        (Actor|DestroyActor)))
    (:CastFailed
      ;[0.15 0.15 0.15 0.5] Damage player on contact
      (bind _asbp_player_controller (Utilities|Casting|CastToBP_PlayerController OtherActor))
      (Default|TakeDamage _asbp_player_controller 4))))

(event EventBeginPlay
  (bind _asbp_pawn_boss (Utilities|Casting|CastToBP_PawnBoss (Actor|GetParentActor)))
  (Variables|Default|SetBoss%20BP _asbp_pawn_boss)
  (bind _asbp_player_controller (Utilities|Casting|CastToBP_PlayerController (Game|GetPlayerCharacter 0)))
  (Variables|Default|SetBP%20Player%20Controller _asbp_player_controller))

(event Collision|EventActorBeginOverlap
  (params (OtherActor :type Actor%20Object%20Reference)))

(event EventTick
  (params (DeltaSeconds :type Float%20%28single-precision%29)))

(fn ConstructionScript)