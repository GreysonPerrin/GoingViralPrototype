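; Boss projectile that homes back toward the boss and hurts the player on the way.
; On BeginPlay it finds the BP_PawnBoss actor and sets its root component as the projectile movement's homing target, after caching the player character as BP_PlayerController.
; Collision overlaps damage the player without destroying the projectile, which despawns when it touches the boss.
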(event OnComponentBeginOverlap(Collision)
  (params (OverlappedComponent :type Primitive%20Component%20Object%20Reference) (OtherActor :type Actor%20Object%20Reference) (OtherComp :type Primitive%20Component%20Object%20Reference) (OtherBodyIndex :type Integer) (bFromSweep :type Boolean) (SweepResult :type Hit%20Result%20Structure%20%28by%20ref%29))
  ;[0.15 0.15 0.15 0.5] Damage player on contact, despawn after touching boss
  (bind _asbp_player_controller (Utilities|Casting|CastToBP_PlayerController OtherActor)
    (:then
      (Default|TakeDamage _asbp_player_controller 4))
    (:CastFailed
      (Utilities|Casting|CastToBP_PawnBoss OtherActor)
      (Actor|DestroyActor))))

(event EventBeginPlay
  (bind _returnvalue (Actor|GetActorOfClass "/Game/MyContent/Blueprints/Enemies/Boss/BP_PawnBoss.BP_PawnBoss_C"))
  (Variables|Default|SetBoss%20BP _returnvalue)
  (bind _asbp_player_controller (Utilities|Casting|CastToBP_PlayerController (Game|GetPlayerCharacter 0)))
  (Variables|Default|SetBP%20Player%20Controller _asbp_player_controller)
  (Variables|/Script/Engine.ProjectileMovementComponent|SetHomingTargetComponent (Variables|Default|GetProjectileMovement) (Variables|/Script/Engine.Actor|GetRootComponent (Variables|Default|GetBoss%20BP))))

(event Collision|EventActorBeginOverlap
  (params (OtherActor :type Actor%20Object%20Reference)))

(event EventTick
  (params (DeltaSeconds :type Float%20%28single-precision%29)))

(fn ConstructionScript)