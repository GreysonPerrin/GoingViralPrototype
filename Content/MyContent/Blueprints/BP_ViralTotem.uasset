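; BP_ViralTotem is a totem actor that destroys itself once its hold counter reaches three.
; Box overlaps with BP_PlayerController toggle PlayerInRange and set that actor's PillarRef to the totem, on exit as well as on entry.
; Each HoldTick call adds one to HoldTime, but nothing in this file calls it or starts its timer.
; Leaving the box clears HoldTimerHandle and resets the count.
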(event OnComponentBeginOverlap(Box)
  (params (OverlappedComponent :type Primitive%20Component%20Object%20Reference) (OtherActor :type Actor%20Object%20Reference) (OtherComp :type Primitive%20Component%20Object%20Reference) (OtherBodyIndex :type Integer) (bFromSweep :type Boolean) (SweepResult :type Hit%20Result%20Structure%20%28by%20ref%29))
  (bind _asbp_player_controller (Utilities|Casting|CastToBP_PlayerController OtherActor))
  (Development|PrintString "Overlapping")
  (Variables|Default|Set%20PlayerInRange true)
  (Variables|/Game/MyContent/Player/BP_PlayerController.BP_PlayerController_C|SetPillarRef _asbp_player_controller self))

(event OnComponentEndOverlap(Box)
  (params (OverlappedComponent :type Primitive%20Component%20Object%20Reference) (OtherActor :type Actor%20Object%20Reference) (OtherComp :type Primitive%20Component%20Object%20Reference) (OtherBodyIndex :type Integer))
  (bind _asbp_player_controller (Utilities|Casting|CastToBP_PlayerController OtherActor))
  (Variables|Default|Set%20PlayerInRange false)
  (Variables|/Game/MyContent/Player/BP_PlayerController.BP_PlayerController_C|SetPillarRef _asbp_player_controller self)
  (Utilities|Time|ClearandInvalidateTimerbyHandle (Variables|Default|GetHoldTimerHandle))
  (Variables|Default|SetHoldTime 0.0))

(event Custom|HoldTick
  (bind _output_get (Variables|Default|SetHoldTime (+ 1.0 (Variables|Default|GetHoldTime))))
  (if (>= _output_get 3.0)
    (Actor|DestroyActor)))

(event EventBeginPlay)

(event Collision|EventActorBeginOverlap
  (params (OtherActor :type Actor%20Object%20Reference)))

(event EventTick
  (params (DeltaSeconds :type Float%20%28single-precision%29)))

(fn ConstructionScript)