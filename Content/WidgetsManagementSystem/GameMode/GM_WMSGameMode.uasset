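; Game mode for a widget management system that opens the main menu at BeginPlay and switches screens, removing cached widgets first.
; CreateWidget builds screens from a widget database, caches them by key and sets the pawn's matching camera state.
; A screen-changed event restores game-only input for one camera state.
; Per-screen looping level sequences with pawn-relative origins, and UI-only input, exist only as unconnected logic.
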(event Custom|OnWidgetScreenChanged_Event
  (bind _playercontroller (Variables|UWM|GetPlayerController))
  ;[0.15 0.15 0.15 0.5] Called everytime a new widget screen is added to viewport, can be extended to execute specific tasks on any screen. At present, inputs are enabled or disabled only.
  (if (Utilities|Enum|Equal(Enum) (CallFunction|GetCameraState (Game|Player|GetPlayerPawn 0)) "NewEnumerator15")
    (Input|EnableInput (Game|Player|GetPlayerPawn 0) _playercontroller)
    (Input|SetInputModeGameOnly _playercontroller true)
    (Variables|/Script/Engine.PlayerController|SetbShowMouseCursor _playercontroller false)))

(event Custom|RemoveOnScreenWidgets
  ;[0.15 0.15 0.15 0.5] Avoid Overlapping Widgets
  (bind _valuepin (Utilities|Map|ForEachLoop(Map) (Variables|Default|GetCachedData))
    (:then
      (Utilities|IsValid (.widgetelement _valuepin)
        (:Is%20Valid
          (Widget|RemovefromParent (.widgetelement _valuepin)))))))

(event Custom|PlayLevelSequenceForCurrentScreen
  (params (ScreenIndex :type Integer))
  ;[0.15 0.15 0.15 0.5] Level Sequences Player
)

(event Custom|OnPause_Event
  ;[0.15 0.15 0.15 0.5] Level Sequences Player
  ;;[0.15 0.15 0.15 0.5] Loop Level Sequence for a screen
  (CallFunction|PlayLevelSequenceforCurrentScreen (Variables|Default|GetCurrentIndex)))

(event EventBeginPlay
  ;[0.15 0.15 0.15 0.5] Cache for future reference
  (Utilities|FlowControl|Sequence
    (:then_0
      (Variables|UWM|SetPlayerController (Game|GetPlayerController 0))
      (EventDispatchers|BindEventtoOnWidgetScreenChanged (EventDispatchers|CreateEvent :!event Custom|OnWidgetScreenChanged_Event)))
    (:then_1
      (Variables|Default|SetCurrentWidgetDB (Variables|/Game/WidgetsManagementSystem/DataAsset/PDA_WidgetData.PDA_WidgetData_C|GetWidgetsData (Variables|UWM|GetWidgetDataBase)))
      ;;[0.15 0.15 0.15 0.5] Create Main Menu on BeginPlay
      (CallFunction|CreateWidget "NewEnumerator3"))))

(event EventAddWidgettoScreen
  (params (Screen :type E_WidgetScreen%20Enum :default "NewEnumerator3"))
  ;[0.15 0.15 0.15 0.5] Add Widgets To Screen
  (CallFunction|RemoveonScreenWidgets)
  (CallFunction|CreateWidget Screen))

(fn ConstructionScript)

(fn CreateWidget
  (params (Key :type E_WidgetScreen%20Enum :default "NewEnumerator3"))
  (bind _cacheddata (Variables|Default|GetCachedData))
  (bind (_value _returnvalue) (Utilities|Map|Find _cacheddata Key))
  (if _returnvalue
    (LocalVariables|SetCurrentScreen (.index _value))
    (UserInterface|Viewport|AddtoViewport (.widgetelement _value) 0)
    (Variables|Default|SetCanPlayLevelSequence? (.playlevelsequence (Utilities|Array|Get(acopy) (Variables|Default|GetCurrentWidgetDB) (LocalVariables|GetCurrentScreen))))
    (CallFunction|ChangeCameraState Key (Game|Player|GetPlayerPawn 0))
    (Variables|Default|SetCurrentLevelSequenceIndex 0)
    (CallFunction|PlayLevelSequenceforCurrentScreen (LocalVariables|GetCurrentScreen))
    (Default|CallOnWidgetScreenChanged)
    (return)
    (else
      (bind (_array_element _array_index) (Utilities|Array|ForEachLoopwithBreak (Variables|Default|GetCurrentWidgetDB) :!label _label)
        (:LoopBody
          (if (Utilities|Enum|Equal(Enum) Key (.WidgetScreen (Utilities|Struct|BreakS_WidgetData _array_element)))
            (LocalVariables|SetCurrentScreen _array_index)
            (goto _label Break)))
        (:Completed
          (if (!= (LocalVariables|GetCurrentScreen) -1)
            (bind _returnvalue_2 (UserInterface|CreateWidget (.widgetelement (Utilities|Array|Get(acopy) (Variables|Default|GetCurrentWidgetDB) (LocalVariables|GetCurrentScreen)))))
            (Utilities|Map|Add (Variables|Default|GetCachedData) Key (Utilities|Struct|MakeS_CacheData (LocalVariables|GetCurrentScreen) _returnvalue_2))
            (UserInterface|Viewport|AddtoViewport _returnvalue_2 0)
            (Variables|Default|SetCanPlayLevelSequence? (.playlevelsequence (Utilities|Array|Get(acopy) (Variables|Default|GetCurrentWidgetDB) (LocalVariables|GetCurrentScreen))))
            (Variables|Default|SetCurrentLevelSequenceIndex 0)
            (CallFunction|PlayLevelSequenceforCurrentScreen (LocalVariables|GetCurrentScreen))
            (CallFunction|ChangeCameraState Key (Game|Player|GetPlayerPawn 0))
            (Default|CallOnWidgetScreenChanged)
            (return)
            (else
              (Development|PrintString "Requested Widget Screen Not found in database" true true "(R=1.000000,G=0.016108,B=0.000000,A=1.000000)")
              (return))))))))